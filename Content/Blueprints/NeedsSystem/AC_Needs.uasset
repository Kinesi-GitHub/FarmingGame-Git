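; AC_Needs is an actor component that tracks its owner's food and water needs.
; Both values decay by fixed rates every tick, unscaled by delta time, and each deals damage through the owner's health component while at or below a low threshold.
; ConsumeItem restores both from DT_FoodItems by matching mesh, though its loop returns after the first found row, match or not.
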(event `self.ReceiveBeginPlay`
  (bind (_valid _return) (`/Game/Vis/BP/HealthAndDamage/Data/VisBP_HealthAndDamage_FL.GetHealth_And_Damage_C` (`self.GetOwner`)))
  ;[1 1 1] BeginPlay
  (if _valid
    (set `self.HealthComponent` _return)
    (else
      (`KismetSystemLibrary.PrintString` (`KismetStringLibrary.BuildString_Object` "" "AC_Needs failed to get health component for " (`self.GetOwner`))))))

(event `self.ReceiveTick`
  (params (DeltaSeconds :type "Float (single-precision)"))
  (bind _healthcomponent (`self.HealthComponent`))
  ;[1 1 1] Mult by delta?
  (`|ExecutionSequence`
    (:`then_0`
      ;[1 1 1] SetNeedDecay
      (set `self.Food` (- (`self.Food`) (`self.FoodDecayRate`)))
      (set `self.Water` (- (`self.Water`) (`self.WaterDecayRate`))))
    (:`then_1`
      ;[1 1 1] ApplyFoodDebuff
      (if (<= (`self.Food`) (`self.LowDebuffStageThreshold`))
        (`/Game/Vis/BP/HealthAndDamage/HealthAndDamage_C.Event_AnyDamage` (`self.HealthComponent`) (`self.GetOwner`) 1.0 null null null)))
    (:`then_2`
      ;[1 1 1] ApplyWaterDebuff
      (if (<= (`self.Water`) (`self.LowDebuffStageThreshold`))
        (`/Game/Vis/BP/HealthAndDamage/HealthAndDamage_C.Event_AnyDamage` _healthcomponent (`self.GetOwner` _healthcomponent) 1.0 null null null)))))

(fn `ConsumeItem`
  (params (Item :type "StaticMesh Object Reference (by ref)"))
  (returns (Ate :type Boolean))
  (locals (names :type "Array of Name"))
  ;[1 1 1] Get the Data for the mesh reference
  (bind _outrownames (`DataTableFunctionLibrary.GetDataTableRowNames` "/Game/Blueprints/NeedsSystem/DT_FoodItems.DT_FoodItems"))
  (bind _output_get (set `local.names` _outrownames))
  (for _array_element _output_get
    (bind _returnvalue (`|GetDataTableRow` "/Game/Blueprints/NeedsSystem/DT_FoodItems.DT_FoodItems" _array_element)
      (:`then`
        (bind (_food _water _mesh) (break `/Game/Blueprints/NeedsSystem/S_NeedItemRowValue` _returnvalue))
        (if (== _mesh Item)
          (set `self.Food` (+ (`self.Food`) _food))
          (set `self.Water` (+ (`self.Water`) _water))
          (return true)
          (else
            (return false)))))))