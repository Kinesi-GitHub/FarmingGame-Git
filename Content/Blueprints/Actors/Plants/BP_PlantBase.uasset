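; BP_PlantBase is a base plant actor that shows growth visually using data from its ACPlantGrowth component.
; UpdateMeshVisuals scales the whole actor uniformly by GrowthAmount, and UpdatePlantGrowthMesh swaps the static mesh to the PlantStructure entry for the current GrowthState.
; Comments intend both updates to reach all clients but question reliance on component replication.
; The authority switch is unwired, and UpdateVisualMeshGrowth is an empty stub.
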(event `UpdateMeshVisuals`
  ;[1 1 1] SendVisualMeshUpdate to all clients
  (`self.SetActorScale3D` (`KismetMathLibrary.Conv_DoubleToVector` (`/Game/Blueprints/Components/AC/AC_PlantGrowth.GrowthAmount` (`self.AC_PlantGrowth`)))))

(event `UpdatePlantGrowthMesh`
  (bind _ac_plantgrowth (`self.AC_PlantGrowth`))
  (bind (_fertilityrequirement _lightsensitivity _lightrequirement _basegrowthrate _temperaturemin _temperaturemaximum _growthstate0 _growthstate1 _growthstate2 _growthstate3) (break `/Game/Blueprints/Components/AC/S_PlantRequirements` (`/Game/Blueprints/Components/AC/AC_PlantGrowth.PlantStructure` _ac_plantgrowth)))
  ;[1 1 1] Update everybody's mesh
  (`StaticMeshComponent.SetStaticMesh` (`self.StaticMesh`) (select `/Game/Blueprints/Components/AC/E_GrowthStage` (`/Game/Blueprints/Components/AC/AC_PlantGrowth.GrowthState` _ac_plantgrowth) :`NewEnumerator0` _growthstate0 :`NewEnumerator1` _growthstate1 :`NewEnumerator2` _growthstate2 :`NewEnumerator3` _growthstate3)))

(fn `UpdateVisualMeshGrowth`)

(fn `UserConstructionScript`)