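; BP_WoodPile is a building-system Blueprint that procedurally stacks a pile of logs as instanced static meshes.
; The construction script calls BuildPile, which clears the instances and places NumLogs in local space along X.
; Every RowLength logs it starts a row higher on Z, with StaggerStack setting that row's starting X to one log spacing.
; The logic to shorten staggered rows is disconnected, so row length stays constant.
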(fn `BuildPile`
  (locals (rowindex :type Integer) (nextLocation :type "Vector Structure") (dynamicRowLength :type Integer))
  (bind (_nextlocation_x _nextlocation_y _nextlocation_z) (`KismetMathLibrary.BreakVector` (`local.nextLocation`)))
  (bind _distancebetweenlogs (`self.DistanceBetweenLogs`))
  (bind (_nextlocation_x_2 _nextlocation_y_2 _nextlocation_z_2) (`KismetMathLibrary.BreakVector` (`local.nextLocation`)))
  (`InstancedStaticMeshComponent.ClearInstances` (`self.InstancedStaticMesh`))
  (set `local.dynamicRowLength` (`self.RowLength`))
  (for _index (range 1 (+ (`self.NumLogs`) 1))
    (`|ExecutionSequence`
      (:`then_0`
        ;[1 1 1] Modulo RowUp
        (if (== (mod (- _index 1) (`local.dynamicRowLength`)) 0)
          (`/Engine/EditorBlueprintResources/StandardMacros.IncrementInt` (`local.rowindex`)
            (:`  `
              (set `local.nextLocation` (`KismetMathLibrary.MakeVector` (`KismetMathLibrary.SelectFloat` _distancebetweenlogs 0.0 (`self.StaggerStack`)) 0.0 (+ _nextlocation_z _distancebetweenlogs)))))))
      (:`then_1`
        ;[1 1 1] Add InstanceHorizontally
        (`InstancedStaticMeshComponent.AddInstance` (`self.InstancedStaticMesh`) (`KismetMathLibrary.MakeTransform` (`local.nextLocation`)) false)
        (set `local.nextLocation` (`KismetMathLibrary.MakeVector` (+ _nextlocation_x_2 (`self.DistanceBetweenLogs`)) 0.0 _nextlocation_z_2))))))

(fn `UserConstructionScript`
  (locals (nextLocation :type "Vector Structure") (rowlength :type Integer :default 7) (rowindex :type Integer :default 1))
  (`parent.UserConstructionScript`)
  (`self.BuildPile`))