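; Actor component for the farming game player that runs a build mode, previewing a placeable actor chosen from inventory.
; Selection inputs step an index into the AC_Inventory item keys to set the active template class.
; While building, Tick spawns one owner-owned preview and moves it to TargetLocation, which is not computed here.
; Primary action checks the item count and removes from inventory, without spawning a placed actor.
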(event `EnhancedInput|/Game/Input/PlayerActions/IA_SelectionUp`
  (params (ActionValue :type Boolean) (ElapsedSeconds :type "Float (double-precision)") (TriggeredSeconds :type "Float (double-precision)") (InputAction :type "InputAction Object Reference" :default "/Game/Input/PlayerActions/IA_SelectionUp.IA_SelectionUp"))
  ;[1 1 1] Selection
  (:`Started`
    (bind _result (`/Engine/EditorBlueprintResources/StandardMacros.IncrementInt` (`self.TemplateIndex`))
      (:`  `
        (set `self.TemplateIndex` _result)
        (`self.UpdateSelection` :!label _label)))))

(event `EnhancedInput|/Game/Input/PlayerActions/IA_SelectionDown`
  (params (ActionValue :type Boolean) (ElapsedSeconds :type "Float (double-precision)") (TriggeredSeconds :type "Float (double-precision)") (InputAction :type "InputAction Object Reference" :default "/Game/Input/PlayerActions/IA_SelectionDown.IA_SelectionDown"))
  ;[1 1 1] Selection
  (:`Started`
    (bind _result (`/Engine/EditorBlueprintResources/StandardMacros.DecrementInt` (`self.TemplateIndex`))
      (:`  `
        (set `self.TemplateIndex` _result)
        (goto _label)))))

(event `self.ReceiveBeginPlay`
  ;[1 1 1] Comment
  (bind _asbp_farming_game_player (cast `/Game/Blueprints/Actors/Pawns/Characters/BP_FarmingGamePlayer` (`self.GetOwner`))) ; change case to allow for other actor types
  (set `self.As BP Farming Game Player` _asbp_farming_game_player))

(event `UpdateSelection`
  (bind _templateindex (`self.TemplateIndex`))
  ;[1 1 1] UpdateSelection
  (bind _keys (`BlueprintMapLibrary.Map_Keys` (`/Game/Blueprints/Components/AC/Inventory/AC_Inventory.Items` (`/Game/Blueprints/Actors/Pawns/Characters/BP_FarmingGamePlayer.AC_Inventory` (`self.As BP Farming Game Player`)))))
  (if (`KismetArrayLibrary.Array_IsValidIndex` _keys _templateindex)
    (set `self.ActiveTemplate` (`|GetArrayItem` _keys _templateindex))))

(event `EnhancedInput|/Game/Input/PlayerActions/IA_Buildmode`
  (params (ActionValue :type Boolean) (ElapsedSeconds :type "Float (double-precision)") (TriggeredSeconds :type "Float (double-precision)") (InputAction :type "InputAction Object Reference" :default "/Game/Input/PlayerActions/IA_Buildmode.IA_Buildmode"))
  ;[1 1 1] Input
  (:`Started`
    (bind _isa (`/Engine/EditorBlueprintResources/StandardMacros.FlipFlop`)
      (:`A`
        _)
      (:`B`
        _))
    (bind _output_get (set `self.Building` _isa))
    (if _output_get
      (`self.UpdateSelection`)
      (else
        (bind _templatereference (`self.TemplateReference`)
          (:`then`
            (`Actor.K2_DestroyActor` _templatereference))
          (:`else`))))))

(event `self.ReceiveTick`
  (params (DeltaSeconds :type "Float (single-precision)"))
  ;[1 1 1] Tick
  (if (`self.Building`)
    (`self.TemplateReference`
      (:`then`
        (`Actor.K2_SetActorLocation` (`self.TemplateReference`) (`self.TargetLocation`) false false :!label _label_2))
      (:`else`
        (bind _activetemplate (`self.ActiveTemplate`)
          (:`then`
            (bind _returnvalue (`|SpawnActorFromClass` _activetemplate (`KismetMathLibrary.MakeTransform` (0.0 0.0 0.0)) "AdjustIfPossibleButAlwaysSpawn" "MultiplyWithRoot" (`self.GetOwner`) (`GameplayStatics.GetPlayerPawn` 0)))
            (set `self.TemplateReference` _returnvalue)
            (goto _label_2))
          (:`else`
            (`KismetSystemLibrary.PrintString` "NoTemplateSelected" true false (struct :`G` 0.66 :`B` 1.0 :`A` 1.0) (`GameplayStatics.GetWorldDeltaSeconds`))))))))

(event `EnhancedInput|/Game/Input/PlayerActions/IA_PrimaryAction`
  (params (ActionValue :type Boolean) (ElapsedSeconds :type "Float (double-precision)") (TriggeredSeconds :type "Float (double-precision)") (InputAction :type "InputAction Object Reference" :default "/Game/Input/PlayerActions/IA_PrimaryAction.IA_PrimaryAction"))
  (bind _ac_inventory (`/Game/Blueprints/Actors/Pawns/Characters/BP_FarmingGamePlayer.AC_Inventory` (`self.As BP Farming Game Player`)))
  (bind (_value _returnvalue) (`BlueprintMapLibrary.Map_Find` (`/Game/Blueprints/Components/AC/Inventory/AC_Inventory.Items` _ac_inventory) (`self.ActiveTemplate`)))
  ;[1 1 1] PrimaryAction
  (:`Started`
    (if _returnvalue
      (if (> _value 0)
        (`/Game/Blueprints/Components/AC/Inventory/AC_Inventory.RemovefromInventory` _ac_inventory)
        (`self.UpdateSelection`)
        (else
          (`KismetSystemLibrary.PrintString` "NotEnough of item"))))))