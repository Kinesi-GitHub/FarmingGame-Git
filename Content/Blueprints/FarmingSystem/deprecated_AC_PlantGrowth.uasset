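; Deprecated plant growth component that advances its owning BP_PlantBase's growth on the server in the farming game.
; Each tick until fully grown, it adds a frame-scaled rate to GrowthAmount, clamped between zero and one.
; The rate combines base growth with a time-of-day daylight level from the farming gamemode, randomized and divided by its timescale.
; GrowthAmount's OnRep sets the plant actor's Z scale; ambient light is a zero stub and the interior check is unwired.
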(event `self.ReceiveBeginPlay`
  ;[1 1 1] BeginPlay
  (`/Engine/EditorBlueprintResources/ActorComponentMacros.Switch Has Authority`
    (:`Authority`
      (bind _asbp_plant_base (cast `/Game/Blueprints/FarmingSystem/Plants/BP_PlantBase` (`self.GetOwner`))
        (:`then`
          (set `self.ParentRef` _asbp_plant_base)
          (bind _asbp_farming_gamemode (cast `/Game/Blueprints/GameLogic/BP_FarmingGamemode` (`GameplayStatics.GetGameMode`)))
          (set `self.As BP Farming Gamemode` _asbp_farming_gamemode))
        (:`CastFailed`
          ;;[1 1 1] In the event this component is attached to a nonPlant actor (might need to be adjusted for animal actors
          (`KismetSystemLibrary.PrintString` "AC_PlantGrowth component not attached to plant actor? "))))))

(event `self.ReceiveTick`
  (params (DeltaSeconds :type "Float (single-precision)"))
  ;[1 1 1] Tick (SERVER ONLY)
  (if (not (`self.FullyGrown`))
    (`/Engine/EditorBlueprintResources/ActorComponentMacros.Switch Has Authority`
      (:`Authority`
        (`|ExecutionSequence`
          (:`then_0`
            (bind _growthrate (`self.GetGrowthRatewithConditions`))
            (set `self.GrowthAmount` (`KismetMathLibrary.FClamp` (+ (* _growthrate DeltaSeconds) (`self.GrowthAmount`))))))))))

(fn `GetAmbientLightLevel`
  (returns (ambientlightlevel :type "Float (double-precision)"))
  (return 0.0))

(fn `GetDayLightLevel`
  (returns (lightlevel :type "Float (double-precision)"))
  (bind _as_bp_farming_gamemode (`self.As BP Farming Gamemode`))
  (bind _timeofday (`/Game/Blueprints/GameLogic/BP_FarmingGamemode.TimeOfDay` _as_bp_farming_gamemode))
  ;[1 1 1] GetDaylight
  (return (select `bool` (`/Game/Blueprints/GameLogic/BP_FarmingGamemode.GetDayTime` _as_bp_farming_gamemode) :`false` (`KismetMathLibrary.MapRangeClamped` _timeofday 12.0 18.0 0.1 0.05) :`true` (`KismetMathLibrary.MapRangeClamped` _timeofday 6.0 12.0 0.0 0.1))))

(fn `GetGrowthRatewithConditions`
  (returns (GrowthRate :type "Float (double-precision)"))
  ;[1 1 1] Main Thread
  (return (* (+ 0.0 (`self.GetDayLightLevel`) (`.BaseGrowthRate_13_2FFFCD9F49974E414982D4A70128FCC9` (break `/Game/Blueprints/FarmingSystem/S_PlantRequirements` (`self.PlantStructure`)))) (`KismetMathLibrary.RandomFloat`) (/ 1.0 (`/Game/Blueprints/GameLogic/BP_FarmingGamemode.Timescale` (`self.As BP Farming Gamemode`))))))

(fn `OnRep_GrowthAmount`
  (`Actor.SetActorScale3D` (`self.ParentRef`) (`KismetMathLibrary.MakeVector` 1.0 1.0 (`self.GrowthAmount`))))