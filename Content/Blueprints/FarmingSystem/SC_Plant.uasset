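; SC_Plant is a farming-system plant component that calculates a plant's growth rate.
; GetFinalGrowthRate adds the daylight level to the base rate from PlantStructure, scales the sum by a random float, and divides it by the farming game mode's Timescale.
; GetDayLightLevel is a stub that returns zero, so daylight currently contributes nothing to growth.
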(fn `GetDayLightLevel`
  (returns (lightlevel :type "Float (double-precision)"))
  (return 0.0))

(fn `GetFinalGrowthRate`
  (returns (ReturnValue :type "Float (double-precision)"))
  (return (* (+ 0.0 (`self.GetDayLightLevel`) (`.BaseGrowthRate_13_2FFFCD9F49974E414982D4A70128FCC9` (break `/Game/Blueprints/FarmingSystem/S_PlantRequirements` (`self.PlantStructure`)))) (`KismetMathLibrary.RandomFloat`) (/ 1.0 (`/Game/Blueprints/GameLogic/BP_FarmingGamemode.Timescale` (`self.As BP Farming Gamemode`))))))