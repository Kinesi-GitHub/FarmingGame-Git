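; AC_PlantGrowth is an actor component that drives plant growth on its owning BP_PlantBase.
; BeginPlay caches the owner; server-side Tick adds growth rate times delta time to GrowthAmount, then calls the plant's visual growth update.
; GrowthState's OnRep refreshes the plant mesh on authority only.
; The condition-based rate and both light-level functions are unfinished stubs with no real calculation, so growth gains nothing from them.
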(event `self.ReceiveBeginPlay`
  ;[1 1 1] BeginPlay
  (bind _asbp_plant_base (cast `/Game/Blueprints/Actors/Plants/BP_PlantBase` (`self.GetOwner`))
    (:`then`
      (set `self.ParentRef` _asbp_plant_base))
    (:`CastFailed`
      ;;[1 1 1] In the event this component is attached to a nonPlant actor (might need to be adjusted for animal actors
      (`KismetSystemLibrary.PrintString` "AC_PlantGrowth component not attached to plant actor? "))))

(event `self.ReceiveTick`
  (params (DeltaSeconds :type "Float (single-precision)"))
  ;[1 1 1] Tick (SERVER ONLY)
  (`/Engine/EditorBlueprintResources/ActorComponentMacros.Switch Has Authority`
    (:`Authority`
      (`|ExecutionSequence`
        (:`then_0`
          (bind _growthrate (`self.GetGrowthRatewithConditions`))
          (bind _output_get (set `self.GrowthRate` _growthrate))
          (set `self.GrowthAmount` (+ (* _output_get DeltaSeconds) (`self.GrowthAmount`))))
        (:`then_1`
          (`/Game/Blueprints/Actors/Plants/BP_PlantBase.UpdateVisualMeshGrowth` (`self.ParentRef`)))))))

(fn `GetAmbientLightLevel`
  (returns (ambientlightlevel :type "Float (double-precision)"))
  (return 0.0))

(fn `GetDayLightLevel`
  (returns (lightlevel :type "Float (double-precision)"))
  ;[1 1 1] GetDaylight
  (return 0.0))

(fn `GetGrowthRatewithConditions`
  (returns (GrowthRate :type "Float (double-precision)"))
  (locals (finalvalue :type "Float (double-precision)"))
  ;[1 1 1] Main Thread
  (`|ExecutionSequence`))

(fn `OnRep_GrowthState`
  (`/Engine/EditorBlueprintResources/ActorComponentMacros.Switch Has Authority` ; if we are the network owner of this actor
    (:`Authority`
      (`/Game/Blueprints/Actors/Plants/BP_PlantBase.UpdatePlantGrowthMesh` (`self.ParentRef`)) ; update the visual mesh for the plant
      (return))))