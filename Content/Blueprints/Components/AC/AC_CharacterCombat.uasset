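; AC_CharacterCombat is a component that gives the farming game player a toggleable lock-on to a target.
; BeginPlay caches the owner as BP_FarmingGamePlayer, the only actor type it supports.
; IA_LockOn flip-flops between sphere-tracing for pawns along the follow camera's forward direction, with debug drawing, and clearing the target.
; While a target is valid, Tick snaps the controller's rotation to face it.
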(event `self.ReceiveTick`
  (params (DeltaSeconds :type "Float (single-precision)"))
  (bind _as_bp_farming_game_player (`self.As BP Farming Game Player`))
  ;[1 1 1] Event Tick
  (`self.Target`
    (:`then`
      (`Controller.SetControlRotation` (`Pawn.GetController` _as_bp_farming_game_player) (`KismetMathLibrary.FindLookAtRotation` (`Actor.K2_GetActorLocation` _as_bp_farming_game_player) (`Actor.K2_GetActorLocation` (`self.Target`)))))
    (:`else`)))

(event `self.ReceiveBeginPlay`
  ;[1 1 1] BeginPlay
  (bind _asbp_farming_game_player (cast `/Game/Blueprints/Actors/Pawns/Characters/BP_FarmingGamePlayer` (`self.GetOwner`))) ; change case to allow for other actor types
  (set `self.As BP Farming Game Player` _asbp_farming_game_player))

(event `EnhancedInput|/Game/Input/PlayerActions/IA_LockOn`
  (params (ActionValue :type Boolean) (ElapsedSeconds :type "Float (double-precision)") (TriggeredSeconds :type "Float (double-precision)") (InputAction :type "InputAction Object Reference" :default "/Game/Input/PlayerActions/IA_LockOn.IA_LockOn"))
  (bind _returnvalue (`Actor.K2_GetActorLocation` (`self.GetOwner`)))
  (:`Started`
    (`/Engine/EditorBlueprintResources/StandardMacros.FlipFlop`
      (:`A`
        ;[1 1 1] LockOn Logic
        (bind (_outhit _returnvalue_2) (`KismetSystemLibrary.SphereTraceSingleForObjects` :`Start` _returnvalue :`End` (+ _returnvalue (* (`KismetMathLibrary.GetForwardVector` (`SceneComponent.K2_GetComponentRotation` (`/Game/Blueprints/Actors/Pawns/Characters/BP_FarmingGamePlayer.FollowCamera` (`self.As BP Farming Game Player`)))) 500.0)) :`Radius` 125.0 :`ObjectTypes` (`|MakeArray` "ObjectTypeQuery3" :!type "EObjectTypeQuery Enum") :`DrawDebugType` "ForDuration"))
        (if _returnvalue_2
          (set `self.Target` (`.HitActor` (`GameplayStatics.BreakHitResult` _outhit)))))
      (:`B`
        ;[1 1 1] NoTargeting
        (set `self.Target` null)))))