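; AC_Inventory is an inventory component whose working part so far is detecting the world item the player looks at.
; Each tick, InteractionTrace sphere-traces forward from the player camera up to InteractionRange, ignoring the owner.
; A newly hit actor is cached as LookAtActor and its LookAtMessage is printed; a miss clears the cache.
; AddToInventory and RemovefromInventory are empty stubs, and LookAt returns an empty string.
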(event `self.ReceiveTick`
  (params (DeltaSeconds :type "Float (single-precision)"))
  ;[1 1 1] Comment
  (`self.InteractionTrace`))

(fn `AddToInventory`)

(fn `InteractionTrace`
  (bind _returnvalue (`GameplayStatics.GetPlayerCameraManager` 0))
  (bind _returnvalue_2 (`Actor.K2_GetActorLocation` _returnvalue))
  (bind (_outhit _returnvalue_3) (`KismetSystemLibrary.SphereTraceSingle` _returnvalue_2 (+ _returnvalue_2 (* (`Actor.GetActorForwardVector` _returnvalue) (`self.InteractionRange`))) 15.0 "TraceTypeQuery3" false (`|MakeArray` (`self.GetOwner`)) "None" true (struct :`R` 1.0 :`A` 1.0) (struct :`G` 1.0 :`A` 1.0) 1.0))
  (if _returnvalue_3
    (bind (_bblockinghit _binitialoverlap _time _distance _location _impactpoint _normal _impactnormal _physmat _hitactor) (`GameplayStatics.BreakHitResult` _outhit))
    (if (!= _hitactor (`self.LookAtActor`))
      (bind _output_get (set `self.LookAtActor` _hitactor))
      (bind _message (message `/Game/Modules/Interfaces/BP_InteractionInterface.LookAt` _output_get))
      (`KismetSystemLibrary.PrintString` (`KismetTextLibrary.Conv_TextToString` _message)))
    (else
      (set `self.LookAtActor` null) ; not looking at anything
    )))

(fn `LookAt`
  (returns (message :type Text))
  (return ""))

(fn `RemovefromInventory`)