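; Item data component that makes its owning world actor a pickup for the inventory system.
; On BeginPlay the authority sets the owner to replicate.
; On StartInteract it finds the activator's AC_Inventory, adds its item row name and quantity, and destroys the owner only if the add succeeds.
; Its LookAt function returns an empty string.
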(event `self.ReceiveBeginPlay`
  ;[1 1 1] BeginPlay
  (`/Engine/EditorBlueprintResources/ActorComponentMacros.Switch Has Authority`
    (:`Authority`
      (`Actor.SetReplicates` (`self.GetOwner`) true))))

(event `/Game/Modules/Interfaces/BP_InteractionInterface.StartInteract`
  (params (CharacterActivator :type "Character Object Reference"))
  (bind _returnvalue (`Actor.GetComponentByClass` CharacterActivator "/Game/Modules/WorldItemInteraction/InventorySystem/AC_Inventory.AC_Inventory_C"))
  ;[1 1 1] Destroy actor upon interaction
  (`/Engine/EditorBlueprintResources/StandardMacros.IsValid` CharacterActivator
    (:`Is Valid`
      (`/Engine/EditorBlueprintResources/StandardMacros.IsValid` _returnvalue
        (:`Is Valid`
          (bind _success (`/Game/Modules/WorldItemInteraction/InventorySystem/AC_Inventory.AddToInventory` _returnvalue (`.RowName` (break `DataTableRowHandle` (`self.ItemID`))) (`self.Quantity`)))
          (if _success
            (`Actor.K2_DestroyActor` (`self.GetOwner`))))))))

(fn `LookAt`
  (returns (message :type Text))
  (return ""))