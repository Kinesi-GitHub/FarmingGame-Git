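; PC_FarmingGamer is the player controller that toggles the inventory menu in a farming game.
; The inventory input action calls ShowMenu, which removes the open W_Menu or, on the local controller, creates one and adds it to the viewport.
; The menu receives player 0's AC_Inventory and an optional target container, so the same event can show another inventory alongside the character's.
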(event `self.ReceiveBeginPlay`)

(event `EnhancedInput|/Game/Input/PlayerActions/IA_InventoryMenu`
  (params (ActionValue :type Boolean) (ElapsedSeconds :type "Float (double-precision)") (TriggeredSeconds :type "Float (double-precision)") (InputAction :type "InputAction Object Reference" :default "/Game/Input/PlayerActions/IA_InventoryMenu.IA_InventoryMenu"))
  ;[1 1 1] OpenInventory
  (:`Started`
    (`self.ShowMenu` null)))

(event `ShowMenu`
  (params (TargetContainer :type "/Game/Modules/WorldItemInteraction/InventorySystem/AC_Inventory Object Reference"))
  (`self.W_Menu`
    (:`then`
      ;[1 1 1] Remove window
      (`Widget.RemoveFromParent` (`self.W_Menu`))
      (set `self.W_Menu` null))
    (:`else`
      (if (`self.IsLocalPlayerController`)
        (bind _returnvalue (`|CreateWidget` "/Game/Modules/GeneralUI/W_Menu.W_Menu_C" null (`self.GetComponentByClass` (`GameplayStatics.GetPlayerCharacter` 0) "/Game/Modules/WorldItemInteraction/InventorySystem/AC_Inventory.AC_Inventory_C") TargetContainer))
        (bind _output_get (set `self.W_Menu` _returnvalue))
        (`UserWidget.AddToViewport` _output_get 0)))))

(fn `UserConstructionScript`)